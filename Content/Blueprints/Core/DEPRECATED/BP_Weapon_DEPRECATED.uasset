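; Deprecated weapon Blueprint that loads its stats, skeletal mesh and material from DT_WeaponTable by weapon name in the construction script.
; TryToFire uses a fire-rate timer handle as the cooldown gate, then picks projectile or trace fire depending on whether a bullet class is set.
; Trace fire only casts a debug-drawn line from the fire arrow, while projectile fire and the ammo-change response are empty stubs.
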(event CallonAmmoChange(BPC_Ammo)
  (params (Ammo :type Integer))
  (if (Utilities|DoesObjectImplementInterface 0 "/Game/Blueprints/Interface/BPI_Info.BPI_Info_C")
    _))

(event Custom|TryToFire
  (if (not (Utilities|Time|IsValidTimerHandle (Variables|Default|GetFireCooldownTimer)))
    (CallFunction|FIreEvent)
    (bind _returnvalue (Utilities|Time|SetTimerbyEvent (delegate Custom|FireCooldawnEnd) (.FireRate (Utilities|Struct|BreakS_WeaponInfo (Variables|Default|GetWeaponInfo)))))
    (Variables|Default|SetFireCooldownTimer _returnvalue)))

(event Custom|FIreEvent
  (if (Utilities|IsValidClass (.BulletClass (Utilities|Struct|BreakS_WeaponInfo (Variables|Default|GetWeaponInfo))))
    (CallFunction|FirebyProjectile)
    (else
      (CallFunction|FirebyTrace))))

(event Custom|FireCooldawnEnd)

(fn ConstructionScript
  (bind _weaponskeletalmesh (Variables|Default|GetWeaponSkeletalMesh))
  (bind _returnvalue (Utilities|GetDataTableRow "/Game/Blueprints/Core/DataTable/DT_WeaponTable.DT_WeaponTable" (Variables|Default|GetNameWeapon))
    (:then
      (Variables|Default|SetWeaponInfo (.WeaponInfo (Utilities|Struct|BreakS_WeaponBody _returnvalue)))
      (Components|SkeletalMesh|SetSkeletalMeshAsset _weaponskeletalmesh (.SkeletalMesh (Utilities|Struct|BreakS_WeaponBody _returnvalue)))
      (Rendering|Material|SetMaterial _weaponskeletalmesh 0 (.MeshMaterial (Utilities|Struct|BreakS_WeaponBody _returnvalue))))))

(fn FirebyTrace
  (bind _arrowfire (Variables|Default|GetArrowFire))
  (bind _returnvalue (Transformation|GetWorldLocation _arrowfire))
  (Collision|LineTraceByChannel _returnvalue (+ _returnvalue (* (Math|Vector|GetForwardVector _arrowfire) 4e+03)) "TraceTypeQuery1" false 0 "ForDuration"))

(fn FirebyProjectile)