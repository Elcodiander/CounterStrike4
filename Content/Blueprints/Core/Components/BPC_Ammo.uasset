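; BPC_Ammo is an ammo component that tracks a bullet count against the weapon info's maximum.
; It fills to the maximum on BeginPlay and offers queries for the current count and empty state.
; ExpenseAmmo sets the count to maximum minus the passed expense, rather than decrementing, then calls the ammo-change notification.
; UpdateAmmo, reached through a client event, and UpdateHealth are stubs returning zero.
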(event Custom|UpdateAmmo_Client
  (params (UpdateAmmo :type Integer))
  (CallFunction|UpdateAmmo UpdateAmmo))

(event EventBeginPlay
  (Service|RecoveryAmmo))

(fn RecoveryAmmo
  (Variables|Default|SetAmmo (Utilities|Struct|BreakS_WeaponInfo (Variables|Default|GetWeaponInfo))))

(fn CurrentAmmo
  (return (Variables|Default|GetAmmo)))

(fn IsEmpty
  (return (== (Variables|Default|GetAmmo) 0)))

(fn ExpenseAmmo
  (params (Expense :type Integer))
  (Variables|Default|SetExpense Expense)
  (bind _output_get (Variables|Default|SetAmmo (- (Utilities|Struct|BreakS_WeaponInfo (Variables|Default|GetWeaponInfo)) (Variables|Default|GetExpense))))
  (if (== _output_get 0)
    (Utilities|FlowControl|DoOnce false
      (:Completed
        _)))
  (Default|CallCallonAmmoChange (Variables|Default|GetAmmo)))

(fn UpdateAmmo
  (params (UpdateAmmo :type Integer))
  (return 0))

(fn UpdateHealth
  (params (UpdateHealth :type Float%20%28double-precision%29))
  (return 0.0))