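; BPC_Health is a health component that tracks Health against MaxHealth and starts at full on BeginPlay through Recovery.
; Damage clamps Health at zero, calls OnDead once through a DoOnce on reaching zero, and calls OnHealthChange.
; AddHealth caps at MaxHealth; neither it nor Recovery calls OnHealthChange.
; UpdateHealth_Client forwards to UpdateHealth, which, like UpdateAmmo, is a stub returning zero.
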(event Custom|UpdateHealth_Client
  (params (UpdateHealth :type Float%20%28double-precision%29))
  (CallFunction|UpdateHealth UpdateHealth))

(event EventBeginPlay
  (Service|Recovery))

(fn CurrentHealth
  (return (Variables|Default|GetHealth)))

(fn IsDead
  (return (== (Variables|Default|GetHealth) 0.0)))

(fn AddHealth
  (params (Add :type Float%20%28double-precision%29))
  (Variables|Default|SetHealth (Math|Float|Min(Float) (+ Add (Variables|Default|GetHealth)) (Variables|Default|GetMax%20Health))))

(fn Damage
  (params (Damage :type Float%20%28double-precision%29))
  (LocalVariables|SetDamageToHealth Damage)
  (bind _output_get (Variables|Default|SetHealth (Math|Float|Max(Float) (- (Variables|Default|GetHealth) (LocalVariables|GetDamageToHealth)) 0.0)))
  (if (== _output_get 0.0)
    (Utilities|FlowControl|DoOnce false
      (:Completed
        (Default|CallOnDead))))
  (Default|CallOnHealthChange _output_get))

(fn Recovery
  (Variables|Default|SetHealth (Variables|Default|GetMax%20Health)))

(fn UpdateAmmo
  (params (UpdateAmmo :type Float%20%28double-precision%29))
  (return 0.0))

(fn UpdateHealth
  (params (UpdateHealth :type Float%20%28double-precision%29))
  (return 0.0))