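; Weapon actor component or actor that loads its stats and mesh from DT_WeaponTable and adds the weapon input mapping for its owning player.
; Fire input runs timer-gated automatic or single shots, playing a montage through BPI_Character.
; Shots spawn BP_Bullet if a bullet class is set, otherwise line-trace for damage, decrementing ammo only on hits.
; Reload instantly refills the magazine; UpdateAmmo and UpdateHealth are stubs.
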(event Custom|TryToFire
  (bind _weaponinfo (Variables|Default|GetWeaponInfo))
  (bind (_firerate _automatic) (Utilities|Struct|BreakS_WeaponInfo _weaponinfo))
  ;[0 0 0] ShootMechanics
  ;;[0 0 0] TryToFire
  (if (not (Utilities|Time|IsTimerActivebyHandle (Variables|Default|GetFire%20Cooldown%20Timer)))
    (if (<= (Utilities|Struct|BreakS_CurrentAditionWeapontInfo (Variables|Default|GetCurrentAdditionWeaponInfo)) 0)
      ;;[1 0.8323 0] Add Sound: EmptyMagazine
      (Development|PrintString "Магазин пуст!")
      (else
        (CallFunction|FIreEvent)
        (if _automatic
          ;;;[0 0 0] AutomaticFire
          (bind _returnvalue (Utilities|Time|SetTimerbyEvent (delegate Custom|AutomaticFire) _firerate true))
          (Variables|Default|SetFire%20Cooldown%20Timer _returnvalue)
          (else
            ;;;[0 0 0] NoAutomaticFire
            (bind _returnvalue_2 (Utilities|Time|SetTimerbyEvent (delegate Custom|FireCooldownEnd) _firerate))
            (Variables|Default|SetFire%20Cooldown%20Timer _returnvalue_2)))))))

(event Custom|FIreEvent
  (bind _ownerpawn (Variables|Default|GetOwnerPawn))
  ;[0 0 0] ShootMechanics
  ;;[0 0 0] FireEvent
  (if (Utilities|DoesObjectImplementInterface _ownerpawn "/Game/Blueprints/UI/BPI_Character.BPI_Character_C")
    (Class|BPICharacter|AnimPlayMontage(Message) _ownerpawn "/Game/FirstPersonArms/Animations/FP_Rifle_Shoot_Montage.FP_Rifle_Shoot_Montage")
    (if (Utilities|IsValidClass (.BulletClass (Utilities|Struct|BreakS_WeaponInfo (Variables|Default|GetWeaponInfo))))
      (CallFunction|FirebyProjectile)
      (else
        (CallFunction|FirebyTrace)))))

(event Custom|FireCooldownEnd
  ;[0 0 0] ShootMechanics
  ;;[0 0 0] TryToFire
  ;;;[0 0 0] NoAutomaticFire
)

(event Custom|AutomaticFire
  ;[0 0 0] ShootMechanics
  ;;[0 0 0] TryToFire
  ;;;[0 0 0] AutomaticFire
  (if (Variables|Default|GetbIsFireButtonPressed)
    (CallFunction|FIreEvent)
    (else
      (Utilities|Time|ClearandInvalidateTimerbyHandle (Variables|Default|GetFire%20Cooldown%20Timer)))))

(event Input|EnhancedActionEvents|EnhancedInputActionIA_Reload
  (params (ActionValue :type Boolean) (ElapsedSeconds :type Float%20%28double-precision%29) (TriggeredSeconds :type Float%20%28double-precision%29) (InputAction :type Input%20Action%20Object%20Reference :default "/Game/FirstPerson/Input/Actions/IA_Reload.IA_Reload"))
  (bind _currentadditionweaponinfo (Variables|Default|GetCurrentAdditionWeaponInfo))
  (bind _currentbullet (Utilities|Struct|BreakS_CurrentAditionWeapontInfo _currentadditionweaponinfo))
  ;[0 0 0] Inputs
  ;;[0 0 0] InputReload
  (:Started
    (Utilities|Struct|SetmembersinS_CurrentAditionWeapontInfo _currentadditionweaponinfo (+ (- (Utilities|Struct|BreakS_WeaponInfo (Variables|Default|GetWeaponInfo)) _currentbullet) _currentbullet))))

(event Input|EnhancedActionEvents|EnhancedInputActionIA_Shoot
  (params (ActionValue :type Boolean) (ElapsedSeconds :type Float%20%28double-precision%29) (TriggeredSeconds :type Float%20%28double-precision%29) (InputAction :type Input%20Action%20Object%20Reference :default "/Game/FirstPerson/Input/Actions/IA_Shoot.IA_Shoot"))
  ;[0 0 0] Inputs
  ;;[0 0 0] InputShoot
  (:Started
    (Variables|Default|SetbIsFireButtonPressed true)
    (CallFunction|TrytoFire))
  (:Completed
    (Variables|Default|SetbIsFireButtonPressed false)))

(event EventBeginPlay
  ;[0 0 0] BeginPlay
  (|CallParentFunction)
  (bind _returnvalue (Utilities|GetDataTableRow "/Game/Blueprints/Core/DataTable/DT_WeaponTable.DT_WeaponTable" (Variables|Default|GetNameWeapon))
    (:then
      (Variables|Default|SetWeaponInfo (.WeaponInfo (Utilities|Struct|BreakS_WeaponBody _returnvalue)))
      (Components|SkeletalMesh|SetSkeletalMeshAsset (.SkeletalMesh (Utilities|Struct|BreakS_WeaponBody _returnvalue)))
      (Rendering|Material|SetMaterial 0 (.MeshMaterial (Utilities|Struct|BreakS_WeaponBody _returnvalue)))
      (bind _aspawn (Utilities|Casting|CastToPawn (Components|GetOwner)))
      (Variables|Default|SetOwnerPawn _aspawn)
      (bind _asplayer_controller (Utilities|Casting|CastToPlayerController (Pawn|GetController _aspawn)))
      (Utilities|IsValid (PlayerController|LocalPlayerSubsystems|GetEnhancedInputLocalPlayerSubsystem _asplayer_controller)
        (:Is%20Valid
          (Input|AddMappingContext (PlayerController|LocalPlayerSubsystems|GetEnhancedInputLocalPlayerSubsystem _asplayer_controller) "/Game/FirstPerson/Input/IMC_Weapons.IMC_Weapons" 1 "(bIgnoreAllPressedKeysUntilRelease=True,bForceImmediately=False,bNotifyUserSettings=False)"))))))

(fn FirebyTrace
  (bind _returnvalue (Transformation|GetSocketLocation "Muzzle"))
  (bind _currentadditionweaponinfo (Variables|Default|GetCurrentAdditionWeaponInfo))
  (bind _ownerpawn (Variables|Default|GetOwnerPawn))
  (bind _currentbullet (Utilities|Struct|BreakS_CurrentAditionWeapontInfo _currentadditionweaponinfo))
  ;[0 0 0] Spawn trace and add him damage
  (bind _outhit (Collision|LineTraceByChannel _returnvalue (+ _returnvalue (* (Math|Vector|GetForwardVector (Pawn|GetControlRotation (Variables|Default|GetOwnerPawn) :!class /Script/Engine.Pawn)) 4e+03)) "TraceTypeQuery3" false 0 "ForDuration"))
  (if (.bBlockingHit (Collision|BreakHitResult _outhit))
    (Game|Damage|ApplyDamage (.HitActor (Collision|BreakHitResult _outhit)) (.Damage (Utilities|Struct|BreakS_WeaponInfo (Variables|Default|GetWeaponInfo))) (Pawn|GetController _ownerpawn) _ownerpawn)
    ;[0 0 0] Checking the trace-bullet in the clip and stopping
    (Utilities|Struct|SetmembersinS_CurrentAditionWeapontInfo _currentadditionweaponinfo (- _currentbullet 1))
    (if (<= _currentbullet 0)
      (Utilities|Time|ClearandInvalidateTimerbyHandle (Variables|Default|GetFire%20Cooldown%20Timer)))))

(fn FirebyProjectile
  (bind _currentadditionweaponinfo (Variables|Default|GetCurrentAdditionWeaponInfo))
  (bind _currentbullet (Utilities|Struct|BreakS_CurrentAditionWeapontInfo _currentadditionweaponinfo))
  ;[0 0 0] Spawn projectile after the shot
  (Game|SpawnActorfromClass "/Game/Blueprints/Core/Weapon/BP_Bullet.BP_Bullet_C" (Math|Transform|MakeTransform (Transformation|GetSocketLocation "Muzzle") (Pawn|GetControlRotation (Variables|Default|GetOwnerPawn) :!class /Script/Engine.Pawn)) "Undefined" "MultiplyWithRoot" 0 (Utilities|Struct|BreakS_WeaponInfo (Variables|Default|GetWeaponInfo)) 0)
  ;[0 0 0] Checking the bullets in the clip and stopping
  (Utilities|Struct|SetmembersinS_CurrentAditionWeapontInfo _currentadditionweaponinfo (- _currentbullet 1))
  (if (<= _currentbullet 0)
    (Utilities|Time|ClearandInvalidateTimerbyHandle (Variables|Default|GetFire%20Cooldown%20Timer))))

(fn UpdateAmmo
  (params (UpdateAmmo :type Integer))
  (return 0))

(fn UpdateHealth
  (params (UpdateHealth :type Float%20%28double-precision%29))
  (return 0.0))