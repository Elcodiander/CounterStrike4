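; Bullet actor that applies damage and an optional effect to whatever it hits, then destroys itself.
; Its Sphere hit event pushes physics-simulating components with an impulse scaled from bullet velocity, then applies DamageOnTap to the hit actor.
; AddEffect constructs an object from the Effect class, if valid, and initializes it on that actor.
; TrySpawnEffect duplicates AddEffect and is not called in this file.
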(event OnComponentHit(Sphere)
  (params (HitComponent :type Primitive%20Component%20Object%20Reference) (OtherActor :type Actor%20Object%20Reference) (OtherComp :type Primitive%20Component%20Object%20Reference) (NormalImpulse :type Vector :default "0, 0, 0") (Hit :type Hit%20Result%20Structure%20%28by%20ref%29))
  (bind _hitactor (Collision|BreakHitResult Hit))
  ;[0 0 0] BulletHit
  (if (Physics|IsSimulatingPhysics OtherComp "None")
    (Physics|AddImpulseatLocation OtherComp (* (Transformation|GetVelocity) 1e+02) (Transformation|GetActorLocation) "None"))
  (Game|Damage|ApplyDamage _hitactor (Variables|Default|GetDamageOnTap) 0 0)
  (CallFunction|AddEffect _hitactor)
  (Actor|DestroyActor))

(fn ConstructionScript)

(fn TrySpawnEffect
  (params (AffectedActor :type Actor%20Object%20Reference))
  (if (Utilities|IsValidClass (Variables|Default|GetEffect))
    (bind _returnvalue (Game|ConstructObjectfromClass (Variables|Default|GetEffect)))
    (Default|InitEffect _returnvalue AffectedActor)))

(fn AddEffect
  (params (AffectedActor :type Actor%20Object%20Reference))
  (bind _effect (Variables|Default|GetEffect))
  (if (Utilities|IsValidClass _effect)
    (bind _returnvalue (Game|ConstructObjectfromClass _effect))
    (Default|InitEffect _returnvalue AffectedActor)))