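; BP_WeaponPickup is a physical weapon pickup that hands its weapon to the character that interacts with it.
; Its mesh and material come from the DT_WeaponTable row matching NameWeapon, applied in the construction script and again in OnRep for replication.
; Interact passes the name and additional weapon info to the character's SpawnWeapon, destroying the pickup only on success.
; InitialImpulse pushes the skeletal mesh with a given impulse.
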(event Custom|InitialImpulse
  (params (Impulse :type Vector))
  (Physics|AddImpulse (Variables|Default|GetPickUpObjectSkeletalMesh) Impulse "None" false))

(event Collision|EventActorBeginOverlap
  (params (OtherActor :type Actor%20Object%20Reference))
  (|CallParentFunction OtherActor) ; This node is disabled and will not be called.\nDrag off pins to build functionality.
)

(event EventInteract
  (params (CharacterPickingUp :type BP%20Character%20Object%20Reference))
  (bind _success (Default|SpawnWeapon CharacterPickingUp (Variables|Default|GetNameWeapon) (Variables|Default|GetCurrent%20Additional%20Weapon%20Info)))
  (if _success
    (Actor|DestroyActor)))

(fn ConstructionScript
  (bind _pickupobjectskeletalmesh (Variables|Default|GetPickUpObjectSkeletalMesh))
  (|CallParentFunction)
  (bind _returnvalue (Utilities|GetDataTableRow "/Game/Blueprints/Core/DataTable/DT_WeaponTable.DT_WeaponTable" (Variables|Default|GetNameWeapon))
    (:then
      (Components|SkeletalMesh|SetSkeletalMeshAsset _pickupobjectskeletalmesh (.SkeletalMesh (Utilities|Struct|BreakS_WeaponBody _returnvalue)))
      (Rendering|Material|SetMaterial _pickupobjectskeletalmesh 0 (.MeshMaterial (Utilities|Struct|BreakS_WeaponBody _returnvalue))))))

(fn OnRepNameWeapon
  (bind _pickupobjectskeletalmesh (Variables|Default|GetPickUpObjectSkeletalMesh))
  (bind _returnvalue (Utilities|GetDataTableRow "/Game/Blueprints/Core/DataTable/DT_WeaponTable.DT_WeaponTable" (Variables|Default|GetNameWeapon))
    (:then
      (Components|SkeletalMesh|SetSkeletalMeshAsset _pickupobjectskeletalmesh (.SkeletalMesh (Utilities|Struct|BreakS_WeaponBody _returnvalue)))
      (Rendering|Material|SetMaterial _pickupobjectskeletalmesh 0 (.MeshMaterial (Utilities|Struct|BreakS_WeaponBody _returnvalue))))))