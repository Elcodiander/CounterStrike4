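; Game state for a Red versus Blue team kill match, tracking the countdown, team scores and player kills and deaths.
; The authority runs a looping one-second timer for the countdown, which at zero prints the winner or draw.
; Multicast events relay time and stat updates to the HUD of each machine's first player controller.
; A kill tagged RedTeam scores for Blue; any other tag scores for Red.
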(event Custom|UpdatePlayerDeaths_Multicast
  (params (PlayerName :type String) (PlayerDeaths :type Integer))
  (bind _returnvalue (Game|GetPlayerController 0))
  (bind _returnvalue_2 (HUD|GetHUD _returnvalue))
  (Utilities|IsValid _returnvalue
    (:Is%20Valid
      (Utilities|IsValid _returnvalue_2
        (:Is%20Valid
          (Class|BPIInfo|UpdatePlayerDeaths(Message) _returnvalue_2 PlayerName PlayerDeaths))))))

(event Custom|UpdatePlayerKills_Multicast
  (params (PlayerName :type String) (PlayerKills :type Integer))
  (bind _returnvalue (Game|GetPlayerController 0))
  (bind _returnvalue_2 (HUD|GetHUD _returnvalue))
  (Utilities|IsValid _returnvalue
    (:Is%20Valid
      (Utilities|IsValid _returnvalue_2
        (:Is%20Valid
          (Class|BPIInfo|UpdatePlayerKills(Message) _returnvalue_2 PlayerName PlayerKills))))))

(event Custom|UpdateGameTime_Multicast
  (params (Time :type Integer))
  (bind _returnvalue (Game|GetPlayerController 0))
  (bind _returnvalue_2 (HUD|GetHUD _returnvalue))
  (Utilities|IsValid _returnvalue
    (:Is%20Valid
      (Utilities|IsValid _returnvalue_2
        (:Is%20Valid
          (Class|BPIInfo|UpdateGameTime(Message) _returnvalue_2 Time))))))

(event Custom|UpdateTeamScore_Multicast
  (params (RedKills :type Integer) (BlueKills :type Integer))
  (bind _returnvalue (Game|GetPlayerController 0))
  (bind _returnvalue_2 (HUD|GetHUD _returnvalue))
  (Utilities|IsValid _returnvalue
    (:Is%20Valid
      (Utilities|IsValid _returnvalue_2
        (:Is%20Valid
          (Class|BPIInfo|UpdateTeamScore(Message) _returnvalue_2 RedKills BlueKills))))))

(event EventBeginPlay
  (Networking|SwitchHasAuthority
    (:Authority
      (Utilities|Time|SetTimerbyEvent (EventDispatchers|CreateEvent :!event UpdateGameTime) 1.0 true))))

(event EventUpdatePlayerDeaths
  (params (PlayerName :type String) (PlayerDeaths :type Integer))
  (CallFunction|UpdatePlayerDeathsMulticast PlayerName PlayerDeaths))

(event EventUpdatePlayerKills
  (params (PlayerName :type String) (PlayerKills :type Integer) (TeamTag :type Name :default "None"))
  (CallFunction|UpdatePlayerKillsMulticast PlayerName PlayerKills)
  (if (== TeamTag "RedTeam")
    (Math|Integer|IncrementInt (Variables|Default|GetBlueKills)
      (:%20%20
        _))
    (else
      (Math|Integer|IncrementInt (Variables|Default|GetRedKills)
        (:%20%20
          _))))
  (CallFunction|UpdateTeamScoreMulticast (Variables|Default|GetRedKills) (Variables|Default|GetBlueKills)))

(fn ConstructionScript)

(fn UpdateGameTime
  (bind _output_get (Variables|Default|SetCountdown (- (Variables|Default|GetCountdown) 1)))
  (CallFunction|UpdateGameTimeMulticast _output_get)
  (if (<= (Variables|Default|GetCountdown) 0)
    (CallFunction|GameEnd)))

(fn GameEnd
  (bind _redkills (Variables|Default|GetRedKills))
  (bind _bluekills (Variables|Default|GetBlueKills))
  (if (== _redkills _bluekills)
    ;[0 0 0] Ничья
    (Development|PrintString "Ничья" true true "(R=0.751524,G=0.863239,B=1.000000,A=1.000000)" 15.0)
    (elif (> _redkills _bluekills)
      (Development|PrintString "Победа Красной команды" true true "(R=1.000000,G=0.000000,B=0.042226,A=1.000000)" 15.0)
      (else
        (Development|PrintString "Победа Синей команды" true true "(R=0.000000,G=0.041733,B=1.000000,A=1.000000)" 15.0)))))