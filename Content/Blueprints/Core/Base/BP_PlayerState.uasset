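; Base PlayerState Blueprint that keeps a player's kill and death counts.
; The PlayerKilled and PlayerDied events increment their counters, then, if the GameState is valid, pass the player name and count to its kill or death message update.
; The kill update also forwards a team tag.
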(event EventBeginPlay)

(event EventPlayerKilled
  (params (TeamTag :type Name :default "None"))
  (bind _returnvalue (Game|GetGameState))
  ;[0 0 0] Event Player Killed
  (bind _result (Math|Integer|IncrementInt (Variables|Default|GetKills))
    (:%20%20
      (Utilities|IsValid _returnvalue
        (:Is%20Valid
          (Class|BPIGameState|UpdatePlayerKills(Message) _returnvalue (PlayerState|GetPlayerName) _result TeamTag))))))

(event EventPlayerDied
  (bind _returnvalue (Game|GetGameState))
  ;[0 0 0] Event Player Died
  (bind _result (Math|Integer|IncrementInt (Variables|Default|GetDeaths))
    (:%20%20
      (Utilities|IsValid _returnvalue
        (:Is%20Valid
          (Class|BPIGameState|UpdatePlayerDeaths(Message) _returnvalue (PlayerState|GetPlayerName) _result))))))

(fn ConstructionScript)